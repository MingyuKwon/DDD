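; Player controller for the Sci-fi UI Pack gameplay demo that puts the gameplay HUD on screen.
; On BeginPlay it resets Health and Energy to their maximums, then creates the gameplay HUD widget, stores it and adds it to the viewport.
; Input mode is then set to game only.
; Despite its name, the health and energy function only initializes those values, and a node enabling the mouse cursor is left unconnected.
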(event EventBeginPlay
  (|AddhealthandEnergybartoviewport_2)
  (bind _returnvalue (UserInterface|CreateWidget "/Game/Sci-fi_UI_Pack/Widget/UIMenuWidget/GameplayMenu/WBP_Sci-fi_UI_Pack_GameplayHUD.WBP_Sci-fi_UI_Pack_GameplayHUD_C"))
  (bind _output_get (Variables|Default|SetGameplay%20HUD%20Scene _returnvalue))
  (UserInterface|Viewport|AddtoViewport _output_get 0)
  (Input|SetInputModeGameOnly self false))

(fn ConstructionScript
  (|CallParentFunction))