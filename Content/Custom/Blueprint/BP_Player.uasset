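; BP_Player is the player Blueprint for a bullet-based battle, routing fire, target-lock and back inputs to BPCBattleUI, which receives the player and five child-actor cameras for two UI stacks.
; The game mode's Stack1To2 event sets the current bullet, defaulting damage to its range midpoint, refreshes the inventory UI and, if input is enabled, switches to stack 2.
; A Tick countdown, held up during animations, gates inputs except right-click back.
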(event Custom|Stack1To2Event_이벤트
  (params (bullet%20Info :type Bullet%20Info%20Structure) (index :type Integer) (bZero :type Boolean))
  (CallFunction|UpdateCurrentBullet bullet%20Info -1 index bZero)
  (CallFunction|UpdateUI)
  (if (Variables|입력|GetbinputEnable)
    (입력|SetInputDisableSecond 0.3)
    (Default|ChangeUIStack (Variables|Default|GetBPC_BattleUI) 2)))

(event EventBeginPlay
  (Utilities|FlowControl|Sequence
    (:then_0
      (Default|InitBattleUIComp (Variables|Default|GetBPC_BattleUI) self (Variables|/Script/Engine.ChildActorComponent|GetChildActor (Variables|Default|GetStack2Index2Camera)) (Variables|/Script/Engine.ChildActorComponent|GetChildActor (Variables|Default|GetStack2Index1Camera)) (Variables|/Script/Engine.ChildActorComponent|GetChildActor (Variables|Default|GetStack2Index0Camera)) (Variables|/Script/Engine.ChildActorComponent|GetChildActor (Variables|Default|GetStack2Index3Camera)) (Variables|/Script/Engine.ChildActorComponent|GetChildActor (Variables|Default|GetStack2Index4Camera)))
      (CallFunction|UpdateUI))
    (:then_1
      (bind _asbp_dddgameplay (Utilities|Casting|CastToBP_DDDGameplay (Game|GetGameMode)))
      (bind _output_get (Variables|Default|SetAs%20BP%20DDDGameplay _asbp_dddgameplay))
      (EventDispatchers|AssignStack1to2Event _output_get (delegate Custom|Stack1To2Event_이벤트)))))

(event EventTick
  (params (DeltaSeconds :type Float%20%28single-precision%29))
  (Variables|Input|SetinputDisableSecond (- (Variables|Input|GetinputDisableSecond) DeltaSeconds))
  (Input|ClampDisableSecond)
  (bind _output_get (Variables|입력|SetbinputEnable (== 0.0 (Variables|Input|GetinputDisableSecond))))
  (if _output_get
    (Development|PrintString "Input Able" true false "(R=0.000000,G=0.660000,B=1.000000,A=1.000000)" 0.0 "1")
    (else
      (Development|PrintString "Input Disable" true false "(R=1.000000,G=0.000000,B=0.028497,A=1.000000)" 0.0 "1"))))

(event Input|KeyboardEvents|SpaceBar
  (params (Key :type Key%20Structure :default "None"))
  (:Pressed
    (if (Variables|입력|GetbinputEnable)
      (Default|ShottoEnemy (Variables|Default|GetBPC_BattleUI)))))

(event Input|KeyboardEvents|A
  (params (Key :type Key%20Structure :default "None"))
  (:Pressed
    (if (Variables|입력|GetbinputEnable)
      (입력|SetInputDisableSecond 0.2)
      (Default|TargetLock (Variables|Default|GetBPC_BattleUI) "NewEnumerator1"))))

(event Input|KeyboardEvents|D
  (params (Key :type Key%20Structure :default "None"))
  (:Pressed
    (if (Variables|입력|GetbinputEnable)
      (입력|SetInputDisableSecond 0.2)
      (Default|TargetLock (Variables|Default|GetBPC_BattleUI) "NewEnumerator2"))))

(event Input|KeyboardEvents|W
  (params (Key :type Key%20Structure :default "None")))

(event Input|MouseEvents|RightMouseButton
  (params (Key :type Key%20Structure :default "None"))
  (:Pressed
    (Default|ChangeUIStack (Variables|Default|GetBPC_BattleUI) 1)))

(fn ConstructionScript)

(fn UpdateCurrentBullet
  (params (bulletInfo :type Bullet%20Info%20Structure) (bulletDamage :type Integer) (inventrotyIndex :type Integer) (bZero :type Boolean))
  (bind (_bufftype _bulletrangemin _bulletrangemax) (Utilities|Struct|BreakBulletInfo bulletInfo))
  (if (== bulletDamage -1)
    (Utilities|Struct|SetmembersinCurrentSetBulletInfo (Variables|Default|GetcurrentSetBulletInfo) bulletInfo (/ (+ _bulletrangemin _bulletrangemax) 2) inventrotyIndex bZero)
    (else
      (Utilities|Struct|SetmembersinCurrentSetBulletInfo (Variables|Default|GetcurrentSetBulletInfo) bulletDamage)))
  (Variables|/Game/Custom/Blueprint/Component/BPC_BattleUI.BPC_BattleUI_C|SetCurrentSetBullet (Variables|Default|GetBPC_BattleUI) (Variables|Default|GetcurrentSetBulletInfo)))

(fn UpdateUI
  (Default|UpdateUIBasedonInventory (Variables|Default|GetBPC_Inventory)))

(fn SetInputDisableSecond
  (params (aimSecond :type Float%20%28double-precision%29))
  (Variables|Input|SetinputDisableSecond (Math|Float|Max(Float) (Variables|Input|GetinputDisableSecond) aimSecond)))

(fn ClampDisableSecond
  (if (Variables|/Game/Custom/GameMode/BP_DDDGameplay.BP_DDDGameplay_C|GetAnimation%20Playing (Variables|Default|GetAs%20BP%20DDDGameplay))
    (Variables|Input|SetinputDisableSecond (Math|Float|Max(Float) (Variables|Input|GetinputDisableSecond) 0.2))
    (else
      (Variables|Input|SetinputDisableSecond (Math|Float|Max(Float) (Variables|Input|GetinputDisableSecond) 0.0)))))