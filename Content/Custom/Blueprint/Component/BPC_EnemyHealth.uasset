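; Enemy health component that tracks an enemy's current health and a stack of skill buffs.
; InitEnemyHealth caches the owner's BPC_EnemyUI component, which receives buffs, current health and max health on each update.
; Skill hits only append to the buff stack, while bullet hits add a damage-derived amount to health after a short delay.
; Health changes are unclamped, with no death handling here.
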(event Custom|HitBySkill
  (params (skillInfo :type Buff%20Structure))
  (Utilities|Array|Add (Variables|Default|GetbuffStack) skillInfo)
  (CallFunction|UpdateEnemyUI))

(event Custom|HitByBullet
  (params (bulletDamage :type Integer))
  (Utilities|FlowControl|Delay 0.5)
  (bind _result (Utilities|NegateInt bulletDamage)
    (:%20%20
      (CallFunction|HealthChange _result)
      (CallFunction|UpdateEnemyUI)
      (Variables|Default|GetEnemyUI
        (:then)
        (:else)))))

(event EventBeginPlay)

(event EventTick
  (params (DeltaSeconds :type Float%20%28single-precision%29)))

(fn UpdateEnemyUI
  (bind _enemyui (Variables|Default|GetEnemyUI)
    (:then
      (Default|UpdateEnemyUI _enemyui (Variables|Default|GetbuffStack) (Variables|Default|GetcurrentHealth) (Variables|Default|GetmaxHealth)))
    (:else)))

(fn InitEnemyHealth
  (Utilities|FlowControl|Sequence
    (:then_0
      (Variables|Default|SetEnemyUI (Actor|GetComponentbyClass (Components|GetOwner) "/Game/Custom/Blueprint/Component/BPC_EnemyUI.BPC_EnemyUI_C"))
      (CallFunction|UpdateEnemyUI))))

(fn HealthChange
  (params (changeAmount :type Integer))
  (Variables|Default|SetcurrentHealth (+ changeAmount (Variables|Default|GetcurrentHealth))))