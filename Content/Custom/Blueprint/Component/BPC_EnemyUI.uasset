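; Enemy UI component that drives a lock-on target widget and a stack/health widget handed to it at initialization.
; TargetLock shows or hides the target widget, slightly enlarges the health widget, and sets the target design for either a bullet or a skill.
; Health, buff and hit updates are forwarded to the health widget.
; On BeginPlay it binds to BP_DDDGameplay's shot-animation event, collapsing a visible target widget when the animation starts.
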(event Custom|ShotAnimationPlaying_이벤트
  (params (bAnimationStart :type Boolean))
  (if bAnimationStart
    (if (Utilities|Enum|Equal(Enum) (Variables|/Script/UMG.Widget|GetVisibility (Variables|UI|GetTarget%20Widget)) "HitTestInvisible")
      (Widget|SetVisibility (Variables|UI|GetTarget%20Widget) "Collapsed"))))

(event EventBeginPlay
  (Utilities|FlowControl|Sequence
    (:then_0
      (bind _asbp_dddgameplay (Utilities|Casting|CastToBP_DDDGameplay (Game|GetGameMode)))
      (Variables|referance|SetAs%20BP%20DDDGameplay _asbp_dddgameplay))
    (:then_1
      (bind _as_bp_dddgameplay (Variables|referance|GetAs%20BP%20DDDGameplay)
        (:then
          (EventDispatchers|AssignShotAnimationPlaying _as_bp_dddgameplay (delegate Custom|ShotAnimationPlaying_이벤트)))
        (:else)))))

(event EventTick
  (params (DeltaSeconds :type Float%20%28single-precision%29)))

(fn IniUIComp
  (params (targetWidget :type WBP%20Target%20Object%20Reference) (stackHealthWidget :type WBP%20Stack%20Health%20Object%20Reference))
  (Variables|UI|SetStack%20Health%20Widget stackHealthWidget)
  (bind _output_get (Variables|UI|SetTarget%20Widget targetWidget))
  (Variables|/Script/UMG.Widget|SetVisibility _output_get "Collapsed"))

(fn TargetLock
  (params (bLockOn :type Boolean) (bSkill :type Boolean) (bulletDamage :type Integer) (skillInfo :type Buff%20Structure))
  (Default|LockonOff (Variables|UI|GetStack%20Health%20Widget) bLockOn bSkill bulletDamage skillInfo)
  (if bLockOn
    (Variables|/Script/UMG.Widget|SetVisibility (Variables|UI|GetTarget%20Widget) "HitTestInvisible")
    (CallFunction|SetUIComponentSize 1.05)
    (if bSkill
      (CallFunction|LockonSkill skillInfo)
      (else
        (CallFunction|LockonBullet bulletDamage)))
    (else
      (Variables|/Script/UMG.Widget|SetVisibility (Variables|UI|GetTarget%20Widget) "Collapsed")
      (CallFunction|SetUIComponentSize 1.0))))

(fn UpdateEnemyUI
  (params (BuffStack :type Array%20of%20Buff%20Structures) (currentHealth :type Integer) (maxHealth :type Integer))
  (Default|UpdateHealthBuff (Variables|UI|GetStack%20Health%20Widget) BuffStack currentHealth maxHealth))

(fn SetUIComponentSize
  (params (widgetScale :type Float%20%28double-precision%29))
  (Widget|Transform|SetRenderScale (Variables|UI|GetStack%20Health%20Widget) (Math|Vector2D|MakeVector2D widgetScale widgetScale)))

(fn LockonBullet
  (params (bulletDamage :type Integer))
  (Default|SetTargetDesign (Variables|UI|GetTarget%20Widget) false bulletDamage "ENone"))

(fn LockonSkill
  (params (skillInfo :type Buff%20Structure))
  (bind (_bufftype _operand) (Utilities|Struct|BreakBuff skillInfo))
  (Default|SetTargetDesign (Variables|UI|GetTarget%20Widget) true _operand _bufftype))

(fn HitbyBulletUIUpdate
  (params (bulletDamage :type Integer))
  (Default|HitbyBullet (Variables|UI|GetStack%20Health%20Widget) bulletDamage false))

(fn HitbyBullet
  (params (bSkill :type Boolean) (bulletDamage :type Integer))
  (Default|HitbyBullet (Variables|UI|GetStack%20Health%20Widget) 0 bSkill))