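; Battle UI component that creates the battle widget and drives a two-stage view: an overview and a per-enemy aiming view.
; Stack changes play widget animations and blend between an overview camera and five per-position cameras chosen by focus index.
; Enemies register by position for left/right target locking, receiving aim previews and delayed bullet or buff shot messages.
; The game mode's shot-animation event re-locks afterwards, or returns to overview when the current bullet is empty.
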(event Custom|Clear%20Target
  (for _array_element (Variables|Default|GetEnemyRegidterArray)
    (Protected|LockOfftoTarget _array_element)))

(event Custom|ShotAnimationPlaying_이벤트
  (params (bAnimationStart :type Boolean))
  (if (not bAnimationStart)
    (if (== (Variables|UI|GetUIStackIndex) 2)
      (if (.bZero (Utilities|Struct|BreakCurrentSetBulletInfo (Variables|TargetData|GetCurrentSetBullet)))
        (액션|ChangeUIStack 1)
        (else
          (Protected|LockontoTarget (Protected|GetEnemyFocusing)))))))

(event Custom|ShotToEnemy
  (bind _focusenemy (Protected|GetEnemyFocusing))
  (if (== (Variables|UI|GetUIStackIndex) 2)
    (Default|CallShotAnimationPlaying (Variables|referance|GetAs%20DDDGame%20Mode) true)
    (Utilities|FlowControl|Delay 0.3)
    (if (Pure|IsDamagettoShot)
      (Class|BPIBattleInteract|ShotBullet(Message) _focusenemy (Pure|BulletDamagetoShot))
      (else
        (Class|BPIBattleInteract|ShotBuff(Message) _focusenemy (Pure|BuffInfotoShot))))))

(event EventBeginPlay
  (bind _returnvalue (Game|GetPlayerController 0))
  (Utilities|FlowControl|Sequence
    (:then_0
      (bind _returnvalue_2 (UserInterface|CreateWidget "/Game/Custom/Widget/GamePlay/WBP_BattleUI.WBP_BattleUI_C"))
      (bind _output_get (Variables|UI|SetBattleUI _returnvalue_2))
      (UserInterface|Viewport|AddtoViewport _output_get 0)
      (Input|SetInputModeGameandUI _returnvalue 0 "DoNotLock" true false)
      (Variables|/Script/Engine.PlayerController|SetbShowMouseCursor _returnvalue true)
      (bind _asbp_dddgameplay (Utilities|Casting|CastToBP_DDDGameplay (Game|GetGameMode)))
      (Variables|referance|SetAs%20DDDGame%20Mode _asbp_dddgameplay))
    (:then_1
      (bind _as_dddgame_mode (Variables|referance|GetAs%20DDDGame%20Mode)
        (:then
          (EventDispatchers|AssignShotAnimationPlaying _as_dddgame_mode (delegate Custom|ShotAnimationPlaying_이벤트)))
        (:else)))))

(event EventBridgeCallLockonOff
  (params (bLockOn :type Boolean) (enemyActor :type Actor%20Object%20Reference))
  (if bLockOn
    (Protected|LockontoTarget enemyActor)
    (else
      (Protected|LockOfftoTarget enemyActor))))

(fn TargetLock
  (params (lockType :type TargetLockType%20Enum :default "NewEnumerator0"))
  (if (== (Variables|UI|GetUIStackIndex) 2)
    (switch Utilities|FlowControl|Switch|SwitchonTargetLockType lockType
      (:NewEnumerator0
        (LocalVariables|SetdefaultUnit 0))
      (:NewEnumerator1
        (LocalVariables|SetdefaultUnit -1))
      (:NewEnumerator2
        (LocalVariables|SetdefaultUnit 1)))
    (Class|BattleUIComponent|FindEnemytoLock (Variables|Default|Getfocus%20Index) (LocalVariables|GetdefaultUnit) (Variables|Default|GetEnemyRegidterArray))))

(fn ChangetoStackUI
  (params (stackIndex :type Integer))
  (LocalVariables|SetShouldPlayAnimation (!= stackIndex (Variables|UI|GetUIStackIndex)))
  (Variables|UI|SetUIStackIndex stackIndex)
  (protected|SetCameraTarget (LocalVariables|GetShouldPlayAnimation)))

(fn InitBattleUIComp
  (params (Stack1Camera :type Actor%20Object%20Reference) (Stack2CameraIndex2 :type Actor%20Object%20Reference) (Stack2CameraIndex1 :type Actor%20Object%20Reference) (Stack2CameraIndex0 :type Actor%20Object%20Reference) (Stack2CameraIndex3 :type Actor%20Object%20Reference) (Stack2CameraIndex4 :type Actor%20Object%20Reference))
  (bind _stack2_camera (Variables|StackCameraTarget|GetStack2%20Camera))
  (Variables|StackCameraTarget|SetStack1%20Camera Stack1Camera)
  (Utilities|Array|Add _stack2_camera Stack2CameraIndex0)
  (Utilities|Array|Add _stack2_camera Stack2CameraIndex1)
  (Utilities|Array|Add _stack2_camera Stack2CameraIndex2)
  (Utilities|Array|Add _stack2_camera Stack2CameraIndex3)
  (Utilities|Array|Add _stack2_camera Stack2CameraIndex4))

(fn EnemyRegister
  (params (positionIndex :type Integer) (EnemyActor :type Actor%20Object%20Reference))
  (bind _returnvalue (Class|BattleUIComponent|RegisterEnemy positionIndex EnemyActor (Variables|Default|GetEnemyRegidterArray)))
  (return _returnvalue))

(fn SetCameraTarget
  (params (bAnimationPlay :type Boolean))
  (switch int (Variables|UI|GetUIStackIndex)
    (:1
      (Game|Player|SetViewTargetwithBlend (Game|GetPlayerController 0) (Variables|StackCameraTarget|GetStack1%20Camera) 0.2 "VTBlend_Cubic" 0.0 false)
      (if bAnimationPlay
        (Default|PlayStack2to1Animation (Variables|UI|GetBattleUI))))
    (:2
      (Game|Player|SetViewTargetwithBlend (Game|GetPlayerController 0) (Utilities|Array|Get(acopy) (Variables|StackCameraTarget|GetStack2%20Camera) (Variables|Default|Getfocus%20Index)) 0.2 "VTBlend_Cubic" 0.0 false)
      (if bAnimationPlay
        (Default|PlayStack1to2Animation (Variables|UI|GetBattleUI))))))

(fn LockOfftoTarget
  (params (lockOffTarget :type Actor%20Object%20Reference))
  (Class|BPIBattleInteract|AimOff(Message) lockOffTarget))

(fn LockontoTarget
  (params (lockOnTarget :type Actor%20Object%20Reference))
  (protected|SetCameraTarget false)
  (Class|BPIBattleInteract|AimonBullet(Message) lockOnTarget (Pure|BulletDamagetoShot) (Pure|BuffInfotoShot)))

(fn GetEnemyFocusing
  (LocalVariables|SetoutputActor (Utilities|Array|Get(acopy) (Variables|Default|GetEnemyRegidterArray) (Variables|Default|Getfocus%20Index)))
  (return (LocalVariables|GetoutputActor)))

(fn UpdateBattleUIBasedonInventory
  (params (EquipBullets :type Array%20of%20Bullet%20Info%20Structures) (RandomBullets :type Array%20of%20Bullet%20Info%20Structures) (bulletLeft :type Integer))
  (Default|UpdateBattleUI (Variables|UI|GetBattleUI) EquipBullets RandomBullets bulletLeft (or (>= bulletLeft (Pure|GetCurrentCost)) (!= (Variables|UI|GetUIStackIndex) 2)))
  (CallFunction|UpdateCurrentBulletUI))

(fn ChangeUIStack
  (params (targetIndex :type Integer))
  (if (!= targetIndex (Variables|UI|GetUIStackIndex))
    (Protected|ChangetoStackUI targetIndex)
    (if (== targetIndex 1)
      (CallFunction|ClearTarget)
      (else
        (Action|TargetLock "NewEnumerator0")))))

(fn UpdateCurrentBulletUI
  (Default|UpdateCurrentBulletUI (Variables|UI|GetBattleUI) (.bulletInfo (Utilities|Struct|BreakCurrentSetBulletInfo (Variables|TargetData|GetCurrentSetBullet)))))

(fn IsDamagettoShot
  (return (Utilities|Enum|Equal(Enum) (.BuffType (Utilities|Struct|BreakBulletInfo (.bulletInfo (Utilities|Struct|BreakCurrentSetBulletInfo (Variables|TargetData|GetCurrentSetBullet))))) "EBullet")))

(fn BuffInfotoShot
  (bind _currentsetbullet (Variables|TargetData|GetCurrentSetBullet))
  (bind (_bulletinfo _currentoperand) (Utilities|Struct|BreakCurrentSetBulletInfo _currentsetbullet))
  (return (Utilities|Struct|MakeBuff (.BuffType (Utilities|Struct|BreakBulletInfo _bulletinfo)) _currentoperand)))

(fn BulletDamagetoShot
  (return (.currentOperand (Utilities|Struct|BreakCurrentSetBulletInfo (Variables|TargetData|GetCurrentSetBullet)))))

(fn GetCurrentCost
  (return (.cost (Utilities|Struct|BreakBulletInfo (.bulletInfo (Utilities|Struct|BreakCurrentSetBulletInfo (Variables|TargetData|GetCurrentSetBullet)))))))