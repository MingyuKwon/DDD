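; BP_EnemyTest is a test enemy actor that registers itself by position index with the player pawn's battle UI component on BeginPlay.
; It then feeds its target and stack-health widgets into BPCEnemyUI and initializes BPCEnemyHealth with that UI component.
; Skill-aim, bullet-aim and aim-off events forward to the UI component's TargetLock, passing skill info or bullet damage when aimed.
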(event EventBeginPlay
  (Utilities|FlowControl|Sequence
    (:then_0
      (bind _output_get (Variables|Default|SetPlayerBattleUI (Actor|GetComponentbyClass (Game|Player|GetPlayerPawn 0) "/Game/Custom/Blueprint/Component/BPC_BattleUI.BPC_BattleUI_C")))
      (Default|EnemyRegister _output_get (Variables|Default|GetpositionIndex) self))
    (:then_1
      (bind _aswbp_target (Utilities|Casting|CastToWBP_Target (UserInterface|GetWidget (Variables|Default|GetTargetWidget))))
      (bind _aswbp_stack_health (Utilities|Casting|CastToWBP_StackHealth (UserInterface|GetWidget (Variables|Default|GetHealthStackWIdget))))
      (Default|IniUIComp (Variables|Default|GetBPC_EnemyUI) _aswbp_target _aswbp_stack_health))
    (:then_2
      (Default|InitEnemyHealthManager (Variables|Default|GetBPC_EnemyHealth) (Variables|Default|GetBPC_EnemyUI)))))

(event EventAimonSkill
  (params (skillInput :type Buff%20Structure))
  (Default|TargetLock (Variables|Default|GetBPC_EnemyUI) true true 0 skillInput))

(event EventTick
  (params (DeltaSeconds :type Float%20%28single-precision%29)))

(event EventAimOff
  (Default|TargetLock (Variables|Default|GetBPC_EnemyUI) false false))

(event EventAimonBullet
  (params (bulletInput :type Integer))
  (Default|TargetLock (Variables|Default|GetBPC_EnemyUI) true false bulletInput))

(fn ConstructionScript)